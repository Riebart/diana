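; ObjectSimConnectorBP bridges simulation objects, keyed by PhysID, to Unreal actors that visualize them.
; New objects spawn a plain Actor with a static mesh component and register it through UpdateExistingVisDataObject.
; Existing objects are moved to the latest position, with linear velocity derived from position and time deltas and angular velocity zeroed.
; Positions and velocities are scaled by half of WorldToMeters; a velocity debug print is disconnected.
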(event EventNewVisDataObject
  (params (PhysID :type Integer) (Position :type Vector))
  (bind _returnvalue (Class|HeadMountedDisplayFunctionLibrary|GetWorldtoMetersScale))
  (bind _returnvalue_2 (/ _returnvalue 2.0))
  (bind _returnvalue_3 (* Position _returnvalue_2))
  (bind _returnvalue_4 (Math|Transform|MakeTransform _returnvalue_3))
  (bind _returnvalue_5 (Game|SpawnActorfromClass "/Script/Engine.Actor" _returnvalue_4 "AlwaysSpawn" 0 0))
  (AddComponent|AddStaticMeshComponent _returnvalue_5 false _returnvalue_4)
  (Class|ObjectSimConnector|UpdateExistingVisDataObject PhysID _returnvalue_5))

(event EventExistingVisDataObject
  (params (PhysID :type Integer) (CurrentPosition :type Vector) (LastPosition :type Vector) (CurrentRealTime :type Float%20%28single-precision%29) (LastRealTime :type Float%20%28single-precision%29) (ActorRef :type Actor%20Object%20Reference))
  (bind _returnvalue (Actor|GetComponentsByClass ActorRef "/Script/Engine.StaticMeshComponent"))
  (bind _returnvalue_2 (- CurrentRealTime LastRealTime))
  (bind _returnvalue_3 (Class|HeadMountedDisplayFunctionLibrary|GetWorldtoMetersScale))
  (bind _item (Utilities|Array|Get(acopy) _returnvalue))
  (bind _returnvalue_4 (/ _returnvalue_3 2.0))
  (if (!= _returnvalue_2 0.0)
    (Transformation|SetActorLocation ActorRef (* CurrentPosition _returnvalue_4) false false)
    (Physics|SetPhysicsLinearVelocity _item (* (/ (- CurrentPosition LastPosition) _returnvalue_2) _returnvalue_4) false "None")
    (Class|PrimitiveComponent|SetPhysicsAngularVelocity _item "0, 0, 0" false "None")))

(fn ConstructionScript)