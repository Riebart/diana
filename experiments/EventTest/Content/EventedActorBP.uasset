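; Event-driven actor that visualises simulated physics objects (USIM) by ID.
; For each new object it spawns an actor with a static mesh at the scaled position and reports the reference back through UpdateExistingVisDataObject.
; For existing objects it moves the actor and sets linear velocity from the position change over elapsed real time, zeroing spin.
; Positions are multiplied by 50 to convert simulation units to Unreal centimetres.
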(event EventNewVisDataObject
  (params (PhysID :type Integer) (Position :type Vector))
  (bind _returnvalue (Math|Float|MakeLiteralFloat 5e+01))
  (bind _returnvalue_2 (* Position _returnvalue))
  (bind _returnvalue_3 (Math|Transform|MakeTransform _returnvalue_2))
  (bind _returnvalue_4 (Game|SpawnActorfromClass "/Script/Engine.Actor" _returnvalue_3 "AlwaysSpawn" 0 0))
  (AddComponent|AddStaticMeshComponent _returnvalue_4 false _returnvalue_3)
  (Class|EventedActor|UpdateExistingVisDataObject PhysID _returnvalue_4))

(event EventExistingVisDataObject
  (params (PhysID :type Integer) (CurrentPosition :type Vector) (LastPosition :type Vector) (CurrentRealTime :type Float%20%28single-precision%29) (LastRealTime :type Float%20%28single-precision%29) (ActorRef :type Actor%20Object%20Reference))
  (bind _returnvalue (Actor|GetComponentsByClass ActorRef "/Script/Engine.StaticMeshComponent"))
  (bind _returnvalue_2 (- CurrentRealTime LastRealTime))
  (bind _returnvalue_3 (Math|Float|MakeLiteralFloat 5e+01))
  (bind _item (Utilities|Array|Get(acopy) _returnvalue))
  (if (!= _returnvalue_2 0.0)
    (Transformation|SetActorLocation ActorRef (* CurrentPosition _returnvalue_3) false false)
    (Physics|SetPhysicsLinearVelocity _item (* (/ (- CurrentPosition LastPosition) _returnvalue_2) _returnvalue_3) false "None")
    (Class|PrimitiveComponent|SetPhysicsAngularVelocity _item "0, 0, 0" false "None")))

(fn ConstructionScript)